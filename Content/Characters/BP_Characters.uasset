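; BP_Characters builds a randomly dressed character from a morph type, or uses a supplied mesh for event characters.
; On BeginPlay it sorts DT_ObjCharacters row indices into hat, glasses, neck and cloth lists.
; CreateCharacters sets the skeletal mesh (every morph currently shares SK_Mannequin_Arms), then, for non-event characters, always adds random cloth and coin-flips the other accessories.
; Each piece takes its mesh and world transform from its table row.
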(event `Set List of obj`
  ;[1 1 1] List of obj
  (bind _outrownames (`DataTableFunctionLibrary.GetDataTableRowNames` "/Game/Data_Table/DT_ObjCharacters.DT_ObjCharacters"))
  (bind _output_get (set `self.List_ObjName` _outrownames))
  (for (_array_element _array_index) _output_get
    (bind _returnvalue (`|GetDataTableRow` "/Game/Data_Table/DT_ObjCharacters.DT_ObjCharacters" _array_element)
      (:`then`
        (switch `/Game/Data_Table/Enum_ObjType` (`.Type_9_8D472ABE482528AD1A154E86BCEA1506` (break `/Game/Data_Table/struc_CharactersObj` _returnvalue))
          (:`NewEnumerator0`
            (`KismetArrayLibrary.Array_Add` (`self.List_Hat`) _array_index))
          (:`NewEnumerator1`
            (`KismetArrayLibrary.Array_Add` (`self.List_Glass`) _array_index))
          (:`NewEnumerator2`
            (`KismetArrayLibrary.Array_Add` (`self.List_Neck`) _array_index))
          (:`NewEnumerator3`
            (`KismetArrayLibrary.Array_Add` (`self.List_Cloth`) _array_index)))))))

(event `Create Characters`
  (params (Morph :type "/Game/Data_Table/Enum_MorphType Enum" :default "NewEnumerator1") (isEvent :type Boolean) (MeshActor :type "SkeletalMesh Object Reference"))
  (bind _skeletalmesh (`self.SkeletalMesh`))
  (bind _staticmeshcloth (`self.StaticMeshCloth`))
  (bind _staticmeshglass (`self.StaticMeshGlass`))
  (bind _staticmeshhat (`self.StaticMeshHat`))
  (bind _staticmeshneck (`self.StaticMeshNeck`))
  (if isEvent
    ;[1 1 1] Event
    (`SkeletalMeshComponent.SetSkeletalMeshAsset` (`self.SkeletalMesh`) MeshActor)
    (else
      ;[1 1 1] Swith morph
      (switch `/Game/Data_Table/Enum_MorphType` Morph
        (:`NewEnumerator1`
          (`SkeletalMeshComponent.SetSkeletalMeshAsset` _skeletalmesh "/Game/FirstPersonArms/Character/Mesh/SK_Mannequin_Arms.SK_Mannequin_Arms"))
        (:`NewEnumerator2`
          (`SkeletalMeshComponent.SetSkeletalMeshAsset` _skeletalmesh "/Game/FirstPersonArms/Character/Mesh/SK_Mannequin_Arms.SK_Mannequin_Arms"))
        (:`NewEnumerator3`
          (`SkeletalMeshComponent.SetSkeletalMeshAsset` _skeletalmesh "/Game/FirstPersonArms/Character/Mesh/SK_Mannequin_Arms.SK_Mannequin_Arms"))
        (:`NewEnumerator4`
          (`SkeletalMeshComponent.SetSkeletalMeshAsset` _skeletalmesh "/Game/FirstPersonArms/Character/Mesh/SK_Mannequin_Arms.SK_Mannequin_Arms"))
        (:`NewEnumerator5`
          (`SkeletalMeshComponent.SetSkeletalMeshAsset` _skeletalmesh "/Game/FirstPersonArms/Character/Mesh/SK_Mannequin_Arms.SK_Mannequin_Arms"))
        (:`NewEnumerator6`
          (`SkeletalMeshComponent.SetSkeletalMeshAsset` _skeletalmesh "/Game/FirstPersonArms/Character/Mesh/SK_Mannequin_Arms.SK_Mannequin_Arms"))
        (:`NewEnumerator0`
          (`SkeletalMeshComponent.SetSkeletalMeshAsset` _skeletalmesh "/Game/FirstPersonArms/Character/Mesh/SK_Mannequin_Arms.SK_Mannequin_Arms"))
        (:`NewEnumerator7`
          (`SkeletalMeshComponent.SetSkeletalMeshAsset` _skeletalmesh "/Game/FirstPersonArms/Character/Mesh/SK_Mannequin_Arms.SK_Mannequin_Arms")))
      ;[1 1 1] Cloth
      (bind _returnvalue (`|GetDataTableRow` "/Game/Data_Table/DT_ObjCharacters.DT_ObjCharacters" (`|GetArrayItem` (`self.List_ObjName`) (`KismetArrayLibrary.Array_Random` (`self.List_Cloth`))))
        (:`then`
          (bind (_type _mesh _transform) (break `/Game/Data_Table/struc_CharactersObj` _returnvalue))
          (`StaticMeshComponent.SetStaticMesh` _staticmeshcloth _mesh)
          (`SceneComponent.K2_SetWorldTransform` _staticmeshcloth _transform false false)
          ;[1 1 1] Glass
          (if (`KismetMathLibrary.RandomBool`)
            (bind _returnvalue_2 (`|GetDataTableRow` "/Game/Data_Table/DT_ObjCharacters.DT_ObjCharacters" (`|GetArrayItem` (`self.List_ObjName`) (`KismetArrayLibrary.Array_Random` (`self.List_Glass`))))
              (:`then`
                (bind (_type_2 _mesh_2 _transform_2) (break `/Game/Data_Table/struc_CharactersObj` _returnvalue_2))
                (`StaticMeshComponent.SetStaticMesh` _staticmeshglass _mesh_2)
                (`SceneComponent.K2_SetWorldTransform` _staticmeshglass _transform_2 false false))))
          ;[1 1 1] Hat
          (if (`KismetMathLibrary.RandomBool`)
            (bind _returnvalue_3 (`|GetDataTableRow` "/Game/Data_Table/DT_ObjCharacters.DT_ObjCharacters" (`|GetArrayItem` (`self.List_ObjName`) (`KismetArrayLibrary.Array_Random` (`self.List_Hat`))))
              (:`then`
                (bind (_type_3 _mesh_3 _transform_3) (break `/Game/Data_Table/struc_CharactersObj` _returnvalue_3))
                (`StaticMeshComponent.SetStaticMesh` _staticmeshhat _mesh_3)
                (`SceneComponent.K2_SetWorldTransform` _staticmeshhat _transform_3 false false))))
          ;[1 1 1] Neck
          (if (`KismetMathLibrary.RandomBool`)
            (bind _returnvalue_4 (`|GetDataTableRow` "/Game/Data_Table/DT_ObjCharacters.DT_ObjCharacters" (`|GetArrayItem` (`self.List_ObjName`) (`KismetArrayLibrary.Array_Random` (`self.List_Neck`))))
              (:`then`
                (bind (_type_4 _mesh_4 _transform_4) (break `/Game/Data_Table/struc_CharactersObj` _returnvalue_4))
                (`StaticMeshComponent.SetStaticMesh` _staticmeshneck _mesh_4)
                (`SceneComponent.K2_SetWorldTransform` _staticmeshneck _transform_4 false false)))))))))

(event `self.ReceiveBeginPlay`
  ;[1 0.9216 0] Begin play
  (`self.Set List of obj`))

(fn `UserConstructionScript`)