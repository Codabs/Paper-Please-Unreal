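; GM_PIS is an unfinished game manager for a document-inspection game with animorph travelers and numbered days.
; NewDay advances the date and resets the timer that Tick accumulates, but day-end and per-date events are empty.
; Create_Character randomly flags good or bad; only good spawns a Visanimorph and randomizes identity from Data_Animorph's "Base" row.
; Visa filling and EntryPermit creation are disconnected, and End_Character is empty.
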(event `NewDay`
  (bind _output_get (set `self.Date` (+ (stale _output_get) 1)))
  (set `self.Day_Timer` 0.0)
  ;[1 1 1] Event ?
  (switch `int` (`self.Date`)))

(event `self.ReceiveTick`
  (params (DeltaSeconds :type "Float (single-precision)"))
  (bind _output_get (set `self.Day_Timer` (+ DeltaSeconds (stale _output_get))))
  (if (> _output_get (`self.Day_Max_Time`))
    _))

(event `Create_Character`
  ;[1 1 1] New character
  ;;[1 1 1] Is he good ?
  (if (> (`KismetMathLibrary.RandomFloat`) 0.5)
    (set `self.IsGood` false)
    (else
      (set `self.IsGood` true)
      (bind _returnvalue (`|SpawnActorFromClass` "/Game/Papers/Visanimorph.Visanimorph_C" (`KismetMathLibrary.Conv_VectorToTransform` (0.0 0.0 0.0)) "Undefined" "OverrideRootScale" null null))
      (bind _returnvalue_2 (`|GetDataTableRow` "/Game/Data_Table/Data_Animorph.Data_Animorph" "Base")
        (:`then`
          (bind (_name _morph _birthdate _gender _id _mat_photo _wheredoeshecomefrom _wherehego _purpose _work _duration) (break `/Game/Data_Table/DataTable_Data_Animorph` _returnvalue_2))
          (bind _output_get (set `self.Name` (`KismetArrayLibrary.Array_Random` _name)))
          (bind _output_get_2 (set `self.Morph` (`KismetArrayLibrary.Array_Random` _morph)))
          (bind _output_get_3 (set `self.Birth_Date` (`KismetArrayLibrary.Array_Random` _birthdate)))
          (bind _output_get_4 (set `self.Gender` (`KismetArrayLibrary.Array_Random` _gender)))
          (bind _output_get_5 (set `self.Weight` (`KismetMathLibrary.Conv_IntToDouble` (`KismetMathLibrary.RandomIntegerInRange` 50 120))))
          (bind _output_get_6 (set `self.Height` (`KismetMathLibrary.Conv_IntToDouble` (`KismetMathLibrary.RandomIntegerInRange` 140 200))))
          (bind _output_get_7 (set `self.Expiration` (`KismetStringLibrary.Concat_StrStr` (`KismetStringLibrary.Conv_IntToString` (`KismetMathLibrary.RandomIntegerInRange` (`self.Date`) 31)) "/05/2449")))
          (bind _output_get_8 (set `self.Id` (`KismetArrayLibrary.Array_Random` _id)))
          (bind _output_get_9 (set `self.Mat_Photo` (`KismetArrayLibrary.Array_Random` _mat_photo)))
          (bind _output_get_10 (set `self.WhereDoesHeComeFrom` (`KismetArrayLibrary.Array_Random` _wheredoeshecomefrom)))
          (bind _output_get_11 (set `self.Where he go` _wherehego))
          (bind _output_get_12 (set `self.Purpose` _purpose))
          (if (not (`KismetStringLibrary.EqualEqual_StrStr` _output_get_12 "Work"))
            (set `self.Work` (`KismetArrayLibrary.Array_Random` _work)))
          (bind _output_get_13 (set `self.Duration` (`KismetArrayLibrary.Array_Random` _duration)))
          (bind _output_get_14 (set `self.EnterBy` (`KismetStringLibrary.Concat_StrStr` (`KismetStringLibrary.Conv_IntToString` (`KismetMathLibrary.RandomIntegerInRange` (`self.Date`) 31)) "/05/2449"))))))))

(event `End_Character`
  ;[1 1 1] End character
)

(fn `UserConstructionScript`)