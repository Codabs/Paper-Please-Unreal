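; BP_BFonction_NextPerson is a button function Blueprint that brings in the next person in a document-check game.
; Its button event caches the player's BP_Pawn and gets the GM_PIS game mode, stopping if either cast fails.
; It then destroys every WorkPass, Visanimorph and EntryPermit actor in the level before asking the game mode to create a new character.
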(event `self.Button Custom Event`
  (bind _asbp_pawn (cast `/Game/Blueprint/BP_Pawn` (`GameplayStatics.GetPlayerPawn` 0)))
  (set `self.As BP Pawn` _asbp_pawn)
  (bind _asgm_pis (cast `/Game/PhysicalS/Misk/GM_PIS` (`GameplayStatics.GetGameMode`)))
  (`self.CleanOtherPaper`)
  (`/Game/PhysicalS/Misk/GM_PIS.Create_Character` :`self` _asgm_pis))

(fn `Button Fonction`
  (`parent.Button Fonction`))

(fn `CleanOtherPaper`
  (bind _outactors (`GameplayStatics.GetAllActorsOfClass` "/Game/Papers/WorkPass.WorkPass_C"))
  (for _array_element _outactors
    (`self.K2_DestroyActor` _array_element))
  (bind _outactors_2 (`GameplayStatics.GetAllActorsOfClass` "/Game/Papers/Visanimorph.Visanimorph_C"))
  (for _array_element_2 _outactors_2
    (`self.K2_DestroyActor` _array_element_2))
  (bind _outactors_3 (`GameplayStatics.GetAllActorsOfClass` "/Game/Papers/EntryPermit.EntryPermit_C"))
  (for _array_element_3 _outactors_3
    (`self.K2_DestroyActor` _array_element_3)))

(fn `UserConstructionScript`
  (`parent.UserConstructionScript`))