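; BP_Whiteboard is a whiteboard that draws onto a render target at the point where it is hit.
; BeginPlay creates a dynamic instance of the WhiteboardMaker material and clears CanvasRenderTarget2D to black.
; The Pickup event converts its hit to a channel 0 UV via FindCollisionUV, prints it and passes it to OnDraw.
; OnDraw sets that UV as the material's LocationToDraw parameter and draws the material into the render target.
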(event `OnDraw`
  (params (LocationToDraw :type "Vector2D Structure"))
  (bind _drawmaterial (`self.DrawMaterial`))
  (`MaterialInstanceDynamic.SetVectorParameterValue` _drawmaterial "LocationToDraw" (`KismetMathLibrary.Conv_VectorToLinearColor` (`KismetMathLibrary.Conv_Vector2DToVector` LocationToDraw 0.1)))
  (`KismetRenderingLibrary.DrawMaterialToRenderTarget` "/Game/Materials/CanvasRenderTarget2D.CanvasRenderTarget2D" _drawmaterial))

(event `/Game/PhysicalS/Misk/i_Pickup.Pickup`
  (params (Accurate :type Boolean) (Hit :type "HitResult Structure") (HideHandIco :type Boolean))
  (bind _uv (`GameplayStatics.FindCollisionUV` Hit))
  (`KismetSystemLibrary.PrintString` (`KismetStringLibrary.Conv_Vector2dToString` _uv))
  (`self.OnDraw` _uv))

(event `self.ReceiveBeginPlay`
  (bind _returnvalue (`KismetMaterialLibrary.CreateDynamicMaterialInstance` "/Game/Materials/WhiteboardMaker.WhiteboardMaker"))
  (set `self.DrawMaterial` _returnvalue)
  (`KismetRenderingLibrary.ClearRenderTarget2D` "/Game/Materials/CanvasRenderTarget2D.CanvasRenderTarget2D"))

(fn `UserConstructionScript`)