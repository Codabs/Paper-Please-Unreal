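; BP_Pawn is a mouse-cursor pawn for dragging Movable components around the world.
; Pressing the left mouse button traces under the cursor and stores the hit component with the grab offset from its origin; releasing clears it.
; Tick deprojects the mouse along its ray by OrginalDistanceTarget, which these graphs never set, and moves the component there minus that offset, without sweeping.
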(event `self.ReceiveBeginPlay`
  (set `PlayerController.bShowMouseCursor` true (`GameplayStatics.GetPlayerController` 0)))

(event `Key|LeftMouseButton`
  (params (Key :type "Key Structure"))
  (bind (_hitresult _returnvalue) (`PlayerController.GetHitResultUnderCursorForObjects` (`GameplayStatics.GetPlayerController` 0) (`self.Object Types`) true))
  (bind (_bblockinghit _binitialoverlap _time _distance _location _impactpoint _normal _impactnormal _physmat _hitactor _hitcomponent) (`GameplayStatics.BreakHitResult` _hitresult))
  (:`Pressed`
    (if _returnvalue
      (if (== (`SceneComponent.Mobility` (`.HitComponent` (`GameplayStatics.BreakHitResult` _hitresult))) (`KismetSystemLibrary.MakeLiteralByte` (enumliteral `EComponentMobility` "Movable")))
        (set `self.Grab Component` _hitcomponent)
        (set `self.Relative Grab Location` (`KismetMathLibrary.InverseTransformLocation` (`KismetMathLibrary.Conv_VectorToTransform` (`SceneComponent.K2_GetComponentLocation` _hitcomponent)) _location)))))
  (:`Released`
    (set `self.Grab Component` null)))

(event `self.ReceiveTick`
  (params (DeltaSeconds :type "Float (single-precision)"))
  (bind (_worldlocation _worlddirection) (`PlayerController.DeprojectMousePositionToWorld` (`GameplayStatics.GetPlayerController` 0)))
  (if (`KismetSystemLibrary.IsValid` (`self.Grab Component`))
    (`SceneComponent.K2_SetWorldLocation` (`self.Grab Component`) (`KismetMathLibrary.InverseTransformLocation` (`KismetMathLibrary.Conv_VectorToTransform` (`self.Relative Grab Location`)) (+ _worldlocation (* _worlddirection (`self.Orginal Distance Target`)))) false false)))

(fn `UserConstructionScript`)