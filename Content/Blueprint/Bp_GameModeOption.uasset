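; Bp_GameModeOption is a helper that hands level-defined spawn points to the GM_PIS game mode.
; On BeginPlay it casts the current game mode to GM_PIS and copies in the world transforms of four referenced actors.
; These set a general spawn transform plus separate ones for entry permit, visa and work pass.
; If the cast fails, nothing is set.
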(event `self.ReceiveBeginPlay`
  (bind _asgm_pis (cast `/Game/PhysicalS/Misk/GM_PIS` (`GameplayStatics.GetGameMode`)))
  (set `/Game/PhysicalS/Misk/GM_PIS.Spawn Transform` (`self.GetTransform` (`self.TransformSpawn`)) _asgm_pis)
  (set `/Game/PhysicalS/Misk/GM_PIS.SpawnTransformOfEntryPermit` (`self.GetTransform` (`self.TransformSpawn_EntryPermit`)) _asgm_pis)
  (set `/Game/PhysicalS/Misk/GM_PIS.SpawnTransformOfVisa` (`self.GetTransform` (`self.TransformSpawn_Visa`)) _asgm_pis)
  (set `/Game/PhysicalS/Misk/GM_PIS.SpawnTransformOfWorkPass` (`self.GetTransform` (`self.TransformSpawn_WorkPass`)) _asgm_pis))

(fn `UserConstructionScript`)