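; BP_Stamp is a stamp actor that the player can pick up.
; On pickup it switches BP_Pawn to its stamp state, passing itself, and disables its static mesh's Visibility and Camera collision responses.
; Each tick a short downward line trace from the static mesh places a plane just above the surface hit.
; PlayAnim plays a non-looping animation on the skeletal mesh.
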(event `self.FonctionOnPickup`
  (bind _asbp_pawn (cast `/Game/Blueprint/BP_Pawn` (`GameplayStatics.GetPlayerPawn` 0)))
  (`/Game/Blueprint/BP_Pawn.GoToStampState` _asbp_pawn self)
  (`self.SetActiveCollision` false))

(event `self.ReceiveTick`
  (params (DeltaSeconds :type "Float (single-precision)"))
  (bind _returnvalue_location (`KismetMathLibrary.BreakTransform` (`SceneComponent.K2_GetComponentToWorld` (`self.StaticMesh`))))
  (bind _returnvalue_location_2 (`KismetMathLibrary.BreakTransform` (`SceneComponent.K2_GetComponentToWorld` (`self.StaticMesh`))))
  (bind (_outhit _returnvalue) (`KismetSystemLibrary.LineTraceSingle` _returnvalue_location_2 (+ _returnvalue_location (0.0 0.0 -30.0)) "TraceTypeQuery1"))
  (if _returnvalue
    (bind (_bblockinghit _binitialoverlap _time _distance _location) (`GameplayStatics.BreakHitResult` _outhit))
    (`SceneComponent.K2_SetWorldLocation` (`self.Plane`) (`KismetMathLibrary.MakeVector` (.x _location) (.y _location) (+ (.z _location) 1.0)) false true)))

(fn `Play Anim`
  (`SkeletalMeshComponent.PlayAnimation` (`self.SkeletalMesh`) null false))

(fn `SetActiveCollision`
  (params (active :type Boolean))
  (if active
    (`PrimitiveComponent.SetCollisionResponseToChannel` (`self.StaticMesh`) "ECC_Visibility" "ECR_Block")
    (`PrimitiveComponent.SetCollisionResponseToChannel` (`self.StaticMesh`) "ECC_Camera" "ECR_Block")
    (else
      (`PrimitiveComponent.SetCollisionResponseToChannel` (`self.StaticMesh`) "ECC_Visibility" "ECR_Ignore")
      (`PrimitiveComponent.SetCollisionResponseToChannel` (`self.StaticMesh`) "ECC_Camera" "ECR_Ignore"))))

(fn `UserConstructionScript`
  (`parent.UserConstructionScript`))