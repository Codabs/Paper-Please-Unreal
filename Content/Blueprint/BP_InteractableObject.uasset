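; Interactable object that highlights and shifts on mouse-over and can be picked up, with an empty FonctionOnPickup event as the hook for pickup behavior.
; Hover enables custom depth and runs a timeline toward an offset and target rotation, while exit or relocation eases it back to its BeginPlay transform.
; Pickup lerps it upward and fires the hook after a short delay.
; IsPickedup blocks hover and repeat pickups until RelocateObject clears it.
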(event `self.ReceiveBeginPlay`
  (`PrimitiveComponent.SetRenderCustomDepth` (`self.StaticMesh`) false)
  (set `self.StartingPosition` (`self.K2_GetActorLocation`))
  (set `self.StartingRotation` (`self.K2_GetActorRotation`)))

(event `/Game/PhysicalS/Misk/i_Pickup.OnMouse`
  (params (Hit :type "HitResult Structure"))
  (bind _returnvalue (`self.K2_GetActorLocation`))
  (bind _returnvalue_2 (`self.K2_GetActorLocation`))
  (if (not (`self.IsPickedup`))
    (`|ExecutionSequence`
      (:`then_0`
        (`PrimitiveComponent.SetRenderCustomDepth` (`self.StaticMesh`) true)
        (bind (_direction _floattimelinezerotoone) (`Timeline|OTo1` :!via `PlayFromStart` :!label _label)
          (:`Update`
            (`self.K2_SetActorLocationAndRotation` (`KismetMathLibrary.VLerp` _returnvalue (+ _returnvalue (`self.OffSetWhenMouseOver`)) _floattimelinezerotoone) (`KismetMathLibrary.RLerp` (`self.K2_GetActorRotation`) (`self.TargetRotationWhenMouseOver`) _floattimelinezerotoone) true true))))
      (:`then_1`
        (bind (_direction_2 _floattimelinezerotoone_2) (`Timeline|Timeline` :!via `Stop` :!label _label_2)
          (:`Update`
            (`self.K2_SetActorLocationAndRotation` (`KismetMathLibrary.VLerp` (`self.K2_GetActorLocation`) (`self.StartingPosition`) _floattimelinezerotoone_2) (`KismetMathLibrary.RLerp` (`self.K2_GetActorRotation`) (`self.StartingRotation`) _floattimelinezerotoone_2) true true))))
      (:`then_2`
        (bind (_direction_3 _floattimelinezerotoone_3) (`Timeline|Timeline_0` :!via `Stop` :!label _label_3)
          (:`Update`
            (`self.K2_SetActorLocation` (`KismetMathLibrary.VLerp` _returnvalue_2 (+ _returnvalue_2 (0.0 0.0 1000.0)) _floattimelinezerotoone_3) true true)))))))

(event `Relocate Object`
  (set `self.IsPickedup` false)
  (`KismetSystemLibrary.Delay` 0.2)
  (`PrimitiveComponent.SetRenderCustomDepth` (`self.StaticMesh`) false :!label _label_4)
  (goto _label_2 :!via `PlayFromStart`))

(event `/Game/PhysicalS/Misk/i_Pickup.ExitMouse`
  (`|ExecutionSequence`
    (:`then_0`
      (goto _label :!via `Stop`))
    (:`then_1`
      (if (not (`self.IsPickedup`))
        (goto _label_4)))))

(event `/Game/PhysicalS/Misk/i_Pickup.Pickup`
  (params (Accurate :type Boolean) (Hit :type "HitResult Structure") (HideHandIco :type Boolean))
  (if (not (`self.IsPickedup`))
    (`|ExecutionSequence`
      (:`then_0`
        (set `self.IsPickedup` true)
        (goto _label_3 :!via `PlayFromStart`))
      (:`then_1`
        (`KismetSystemLibrary.Delay` 0.2)
        (`self.FonctionOnPickup`)))))

(event `FonctionOnPickup`)

(fn `SetCollision`)

(fn `UserConstructionScript`)