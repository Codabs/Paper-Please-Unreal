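; BP_Button is an interactable button actor that triggers a set of linked objects.
; On Pickup, if CanHitTheButton is set, it loops through the ButtonFonction array and calls ButtonCustomEvent and ButtonFonction on each element.
; OnMouse and ExitMouse toggle custom depth rendering on its static mesh as a hover highlight, which starts off at BeginPlay.
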(event `self.ReceiveBeginPlay`
  (`PrimitiveComponent.SetRenderCustomDepth` (`self.StaticMesh`) false))

(event `/Game/PhysicalS/Misk/i_Pickup.Pickup`
  (params (Accurate :type Boolean) (Hit :type "HitResult Structure") (HideHandIco :type Boolean))
  (if (`self.canHitTheButton`)
    (if (`KismetArrayLibrary.Array_IsValidIndex` (`self.ButtonFonction`))
      (for _array_element (`self.ButtonFonction`)
        (`/Game/Blueprint/BP_ButtonFonction.Button Custom Event` _array_element)
        (`/Game/Blueprint/BP_ButtonFonction.Button Fonction` _array_element)))))

(event `/Game/PhysicalS/Misk/i_Pickup.OnMouse`
  (params (Hit :type "HitResult Structure"))
  (`PrimitiveComponent.SetRenderCustomDepth` (`self.StaticMesh`) true))

(event `/Game/PhysicalS/Misk/i_Pickup.ExitMouse`
  (`PrimitiveComponent.SetRenderCustomDepth` (`self.StaticMesh`) false))

(fn `UserConstructionScript`)